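; Gravity gun weapon actor that can be picked up and dropped, and plays feedback for grabbing and launching objects.
; ObjectGrabber events turn the HUD crosshair green when a grab is possible and play grab and release sounds.
; ObjectLauncher events play sound, camera shake and explosion effects on success, or a zap and brief sparks on failure.
; Pickup attaches the gun to a socket; Drop restores physics and re-enables capsule queries after a delay.
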(event `self.ObjectGrabber.OnCanGrabChanged`
  (params (CanGrab :type Boolean))
  ;[1 1 1] Objectgrabber Eventhandlers
  (bind _asbp_gravity_hud (cast `/Game/Blueprints/BP_GravityHUD` (`PlayerController.GetHUD` (`GameplayStatics.GetPlayerController` 0))))
  (set `/Game/Blueprints/BP_GravityHUD.bUseGreenCosshair` CanGrab _asbp_gravity_hud))

(event `self.ObjectGrabber.OnGrab`
  ;[1 1 1] Objectgrabber Eventhandlers
  (`GameplayStatics.PlaySound2D` "/Game/Assets/Audio/HL2_Sounds/physcannon_pickup.physcannon_pickup" 1.0 1.0 0.0 null null))

(event `self.ObjectGrabber.OnRelease`
  ;[1 1 1] Objectgrabber Eventhandlers
  (`GameplayStatics.PlaySound2D` "/Game/Assets/Audio/HL2_Sounds/physcannon_drop.physcannon_drop" 1.0 1.0 0.0 null null))

(event `self.ObjectLauncher.OnLaunchSuccess`
  (bind _p_explosion (`self.P_Explosion`))
  ;[1 1 1] ObjectLauncher Eventhandlers
  (`|ExecutionSequence`
    (:`then_0`
      (`GameplayStatics.PlaySound2D` "/Game/Assets/Audio/HL2_Sounds/superphys_launch1.superphys_launch1" 1.0 1.0 0.0 null null))
    (:`then_1`
      (`GameplayStatics.PlayWorldCameraShake` "/Game/Blueprints/BP_CameraShake.BP_CameraShake_C" (`self.K2_GetActorLocation`) 0.0 500.0 0.0)
      (`SceneComponent.SetHiddenInGame` _p_explosion false false)
      (`ActorComponent.Activate` _p_explosion true))))

(event `self.ObjectLauncher.OnLaunchFail`
  ;[1 1 1] ObjectLauncher Eventhandlers
  (`|ExecutionSequence`
    (:`then_0`
      (`GameplayStatics.PlaySound2D` "/Game/Assets/Audio/HL2_Sounds/superphys_small_zap1.superphys_small_zap1" 1.0 1.0 0.0 null null)
      (`SceneComponent.SetHiddenInGame` (`self.P_Sparks1`) false false)
      (`KismetSystemLibrary.Delay` 0.3)
      (`SceneComponent.SetHiddenInGame` (`self.P_Sparks1`) true false))))

(event `Event Drop`
  ;[1 1 1] Gun pickup and drop events
  (`self.K2_DetachFromActor` "KeepWorld" "KeepWorld" "KeepWorld")
  (`PrimitiveComponent.SetSimulatePhysics` (`self.Box`) true)
  (`KismetSystemLibrary.Delay` 1.0)
  (`PrimitiveComponent.SetCollisionEnabled` (`self.Capsule`) "QueryOnly"))

(event `Event Pickup`
  (params (ComponentToAttachTo :type "SceneComponent Object Reference") (SocketName :type Name))
  ;[1 1 1] Gun pickup and drop events
  (`PrimitiveComponent.SetSimulatePhysics` (`self.Box`) false)
  (`PrimitiveComponent.SetCollisionEnabled` (`self.Capsule`) "NoCollision")
  (`self.K2_AttachToComponent` ComponentToAttachTo SocketName "SnapToTarget" "SnapToTarget" "KeepRelative"))

(fn `UserConstructionScript`)